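; First-person character Blueprint with a hold-to-grapple hook that pulls the player toward the surface they aim at.
; Pressing the fire input line-traces from the camera; a hit stores the grab point, switches movement to Flying and shows the cable.
; While grappling, Tick pins the cable end to that point and applies force toward it, nudged sideways by axis input.
; Releasing restores Falling and hides the cable.
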(event `InputAction|Fire Grapping Hook`
  (params (Key :type "Key Structure"))
  (bind _firstpersoncameracomponent (`self.FirstPersonCameraComponent`))
  (bind _returnvalue (`SceneComponent.K2_GetComponentLocation` _firstpersoncameracomponent))
  ;[1 1 1] Grappling Mechanic
  (:`Pressed`
    (bind (_outhit _returnvalue_2) (`KismetSystemLibrary.LineTraceSingle` :`Start` _returnvalue :`End` (+ (* (`KismetMathLibrary.GetForwardVector` (`SceneComponent.K2_GetComponentRotation` _firstpersoncameracomponent)) 3000.0) _returnvalue) :`TraceChannel` "TraceTypeQuery1" :`DrawDebugType` "ForDuration"))
    (if _returnvalue_2
      (set `self.GrabPoint` (`.ImpactPoint` (`GameplayStatics.BreakHitResult` _outhit)))
      (set `self.isGrappling` true)
      (`CharacterMovementComponent.SetMovementMode` (`self.CharacterMovement`) "MOVE_Flying" 0)
      (`SceneComponent.SetVisibility` (`self.Cable`) true false)))
  (:`Released`
    (set `self.isGrappling` false)
    (`CharacterMovementComponent.SetMovementMode` (`self.CharacterMovement`) "MOVE_Falling" 0)
    (`SceneComponent.SetVisibility` (`self.Cable`) false false)))

(event `self.ReceiveTick`
  (params (DeltaSeconds :type "Float (single-precision)"))
  (if (`self.isGrappling`)
    (set `CableComponent.EndLocation` (`KismetMathLibrary.InverseTransformLocation` (`self.GetTransform`) (`self.GrabPoint`)) (`self.Cable`))
    (`CharacterMovementComponent.AddForce` (`self.CharacterMovement`) (* (`KismetMathLibrary.Normal` (+ (`KismetMathLibrary.GetDirectionUnitVector` (`self.K2_GetActorLocation`) (`self.GrabPoint`)) (* (* (`self.GetActorRightVector`) (`self.GetInputAxisKeyValue`)) 0.1))) 250000.0))))

(fn `UserConstructionScript`
  (`parent.UserConstructionScript`))